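; Runner character Blueprint for a lane-based runner, handling lane switches, game over and power-up feedback.
; ChangeLane restarts a timeline that feeds its lane value to ChangeLaneUpdate and calls ChangeLaneFinished at the end, both defined outside this graph.
; GameOver shows the end widget and cursor after a short delay, while PowerEffect spawns a potion particle at SpawnPoint.
; Despite its name, RagDollPhysics turns mesh physics simulation off and disables movement.
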(event EventChangeLane
  (bind _lanevalue (Timeline|LaneSwitchingTimeline PlayFromStart)
    (:Update
      (Class|Runner|ChangeLaneUpdate _lanevalue))
    (:Finished
      (Class|Runner|ChangeLaneFinished))))

(event EventGameOver
  (Utilities|FlowControl|Delay 0.5)
  (bind _returnvalue (UserInterface|CreateWidget "/Game/_Game/Blueprints/Game_End.Game_End_C"))
  (UserInterface|Viewport|AddtoViewport _returnvalue 0)
  (Variables|/Script/Engine.PlayerController|SetbShowMouseCursor (Game|GetPlayerController 0) true))

(event EventPowerEffect
  (Effects|SpawnEmitteratLocation "/Game/InfinityBladeEffects/Effects/FX_Ability/Heal/P_Heal_Potion.P_Heal_Potion" (Transformation|GetWorldLocation (Variables|Default|GetSpawnPoint))))

(fn ConstructionScript)

(fn RagDollPhysics
  (Physics|SetSimulatePhysics (Variables|Character|GetMesh) false)
  (Pawn|Components|CharacterMovement|DisableMovement (Variables|Character|GetCharacterMovement)))